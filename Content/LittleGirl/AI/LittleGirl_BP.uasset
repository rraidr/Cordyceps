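; LittleGirl_BP is the Blueprint for a little girl AI pawn that follows the player's third-person character.
; On BeginPlay it caches the player character, then starts a self-repeating FollowPlayer event on a 0.2 second delay.
; Each pass issues AI MoveTo toward the player while the follow flag is set and the gap is wide enough.
; Otherwise it targets itself with the move, so it holds position.
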(event Custom|Follow%20Player
  (if (and (Variables|Default|GetfollowPlayer?) (>= (Transformation|GetDistanceTo (Variables|Default|GetCharacter)) 2e+02))
    (AI|AIMoveTo self "0, 0, 0" (Variables|Default|GetCharacter) 5.0 false
      (:then
        _))
    (else
      (AI|AIMoveTo self "0, 0, 0" self 5.0 false
        (:then
          _))))
  (Utilities|FlowControl|Delay 0.2)
  (CallFunction|FollowPlayer))

(event EventBeginPlay
  (bind _asthird_person_character (Utilities|Casting|CastToThirdPersonCharacter (Game|GetPlayerCharacter 0)))
  (Variables|Default|SetCharacter _asthird_person_character)
  (CallFunction|FollowPlayer))

(fn ConstructionScript)