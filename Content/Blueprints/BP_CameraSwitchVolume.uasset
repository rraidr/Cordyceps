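; BP_CameraSwitchVolume is a trigger volume that switches the player's view to another camera when the third-person character enters it.
; OverlapCollision's begin overlap casts to ThirdPersonCharacter, gets its PlayerController and calls SetViewTargetWithBlend on CameraToFind.
; End overlap does nothing: the logic that would return the view to the character is disconnected, so leaving the volume keeps the switched camera.
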(event OnComponentBeginOverlap(OverlapCollision)
  (params (OverlappedComponent :type Primitive%20Component%20Object%20Reference) (OtherActor :type Actor%20Object%20Reference) (OtherComp :type Primitive%20Component%20Object%20Reference) (OtherBodyIndex :type Integer) (bFromSweep :type Boolean) (SweepResult :type Hit%20Result%20Structure%20%28by%20ref%29))
  (bind _asthird_person_character (Utilities|Casting|CastToThirdPersonCharacter OtherActor))
  (if (Utilities|IsValid _asthird_person_character)
    (bind _asplayer_controller (Utilities|Casting|CastToPlayerController (Pawn|GetController _asthird_person_character)))
    (if (Utilities|IsValid _asplayer_controller)
      (Game|Player|SetViewTargetwithBlend _asplayer_controller (Variables|Default|GetCameraToFind) 0.0 "VTBlend_Linear" 0.0 false))))

(event OnComponentEndOverlap(OverlapCollision)
  (params (OverlappedComponent :type Primitive%20Component%20Object%20Reference) (OtherActor :type Actor%20Object%20Reference) (OtherComp :type Primitive%20Component%20Object%20Reference) (OtherBodyIndex :type Integer)))

(event EventBeginPlay)

(event Collision|EventActorBeginOverlap
  (params (OtherActor :type Actor%20Object%20Reference)))

(event EventTick
  (params (DeltaSeconds :type Float%20%28single-precision%29)))

(fn ConstructionScript)