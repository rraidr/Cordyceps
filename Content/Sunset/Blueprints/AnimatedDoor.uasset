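; AnimatedDoor is a key-locked double door that the player opens and closes with E while inside its trigger box.
; Box overlap enables and disables player input, and HasKey, which is not set here, gates the key press.
; The DoorRotation timeline swings DoorL and DoorR in mirrored yaw, playing or reversing according to DoorClosed.
; Tick derives DoorClosed each frame from the timeline's DoorOpen value.
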(event OnComponentBeginOverlap(Box)
  (params (OverlappedComponent :type Primitive%20Component%20Object%20Reference) (OtherActor :type Actor%20Object%20Reference) (OtherComp :type Primitive%20Component%20Object%20Reference) (OtherBodyIndex :type Integer) (bFromSweep :type Boolean) (SweepResult :type Hit%20Result%20Structure%20%28by%20ref%29))
  (Input|EnableInput (Game|GetPlayerController 0)))

(event OnComponentEndOverlap(Box)
  (params (OverlappedComponent :type Primitive%20Component%20Object%20Reference) (OtherActor :type Actor%20Object%20Reference) (OtherComp :type Primitive%20Component%20Object%20Reference) (OtherBodyIndex :type Integer))
  (Input|DisableInput (Game|GetPlayerController 0)))

(event EventTick
  (params (DeltaSeconds :type Float%20%28single-precision%29))
  (Variables|Default|SetDoorClosed (< (stale Input|KeyboardEvents|E _door_open) 1.0)))

(event Input|KeyboardEvents|E
  (params (Key :type Key%20Structure :default "None"))
  (:Pressed
    (if (Variables|Default|GetHasKey)
      (if (Variables|Default|GetDoorClosed)
        (bind _door_open (Timeline|Door%20Rotation Play)
          (:Update
            (Transformation|SetRelativeLocationAndRotation (Variables|Default|GetDoorL) "-80.000000, 0, 0" (Math|Rotator|MakeRotator 0.0 0.0 _door_open) false false)
            (Transformation|SetRelativeLocationAndRotation (Variables|Default|GetDoorR) "80.000000, 0, 0" (* (Math|Rotator|MakeRotator 0.0 0.0 _door_open) -1.0) false false)))
        (else
          (Timeline|Door%20Rotation Reverse))))))

(fn ConstructionScript)